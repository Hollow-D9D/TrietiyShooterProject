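; AI controller for zombie enemies that runs the BT_AIZombie behavior tree on BeginPlay.
; Each Tick it compares the pawn's distance to player 0 against fixed thresholds to choose between idle, chase and attack flags.
; It writes those flags to the Blackboard, along with stun and death state read from the controlled BP_EnemyBase, for the tree to consume.
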(event `self.ReceiveBeginPlay`
  (`self.RunBehaviorTree` "/Game/Blueprints/AI/BT_AIZombie.BT_AIZombie"))

(event `self.ReceiveTick`
  (params (DeltaSeconds :type "Float (single-precision)"))
  (bind _returnvalue (`AIBlueprintHelperLibrary.GetBlackboard` null))
  (bind _returnvalue_2 (`KismetMathLibrary.Vector_Distance` (`self.K2_GetActorLocation` (`self.K2_GetPawn`)) (`self.K2_GetActorLocation` (`GameplayStatics.GetPlayerPawn` 0))))
  (`|ExecutionSequence`
    (:`then_0`
      (if (> _returnvalue_2 1000.0)
        (set `self.ShouldChase` false)
        (set `self.ShouldAttack` false)
        (elif (> _returnvalue_2 100.0)
          (set `self.ShouldChase` true)
          (set `self.ShouldAttack` false)
          (else
            (set `self.ShouldAttack` true)
            (set `self.ShouldChase` false)))))
    (:`then_1`
      (`BlackboardComponent.SetValueAsBool` _returnvalue "ShouldChase" (`self.ShouldChase`))
      (`BlackboardComponent.SetValueAsBool` _returnvalue "ShouldAttack" (`self.ShouldAttack`))
      (bind _asbp_enemy_base (cast `/Game/Blueprints/BP_EnemyBase` (`self.K2_GetPawn`)))
      (`BlackboardComponent.SetValueAsBool` _returnvalue "ShouldStun" (`/Game/Blueprints/BP_EnemyBase.IsStunned` _asbp_enemy_base))
      (`BlackboardComponent.SetValueAsBool` _returnvalue "IsDead" (`/Game/Blueprints/BP_EnemyBase.IsDie` _asbp_enemy_base)))))

(fn `UserConstructionScript`)