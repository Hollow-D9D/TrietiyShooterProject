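; Base enemy Blueprint that handles how enemies react to different projectile types and die.
; TakeDamage switches on projectile type: Pistol only sets the stun flag, Laser drains the BPHealth component until death, and BFG kills instantly.
; Die sets a death flag and plays a sound at the capsule, while only the BFG path also destroys the actor.
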(event `self.ReceiveTick`
  (params (DeltaSeconds :type "Float (single-precision)"))
  (`parent.ReceiveTick` DeltaSeconds))

(fn `BFGDeath`
  (`self.Die`)
  (`self.K2_DestroyActor`))

(fn `Die`
  (set `self.IsDie` true)
  (`GameplayStatics.PlaySoundAtLocation` (`self.DeathSound`) (`SceneComponent.K2_GetComponentLocation` (`self.CapsuleComponent`)) (struct) 1.0 1.0 0.0 null null null null))

(fn `TakeDamage`
  (params (DamageAmount :type Integer) (ProjectileType :type "/Game/Blueprints/EProjectileType Enum" :default "NewEnumerator0"))
  (bind _bp_health (`self.BP_Health`))
  (switch `/Game/Blueprints/EProjectileType` ProjectileType
    (:`NewEnumerator0`
      (set `self.IsStunned` true))
    (:`NewEnumerator1`
      (`/Game/Blueprints/HealthBP/BP_Health.TakeDamage` _bp_health DamageAmount)
      (if (<= (`/Game/Blueprints/HealthBP/BP_Health.Health` _bp_health) 0)
        (`self.Die`)))
    (:`NewEnumerator2`
      (`self.BFGDeath`))))

(fn `UserConstructionScript`
  (`parent.UserConstructionScript`))