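; BP_Start_Door is a door actor that swings open and shows a text label when something is near it.
; A Box trigger's begin and end overlaps set the NeartheDoor flag and toggle the TextRender's visibility, without filtering the overlapping actor.
; The OpenDoor event plays a Timeline that lerps component I's relative rotation through a quarter turn.
; Nothing in this Blueprint calls OpenDoor, reads the flag or closes the door.
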(event `Open Door`
  (bind (_direction _newtrack_0) (`Timeline|Timeline`)
    (:`Update`
      (`SceneComponent.K2_SetRelativeRotation` (`self.I`) (`KismetMathLibrary.RLerp` (struct) (struct :`Yaw` 90.0) _newtrack_0) false false))))

(event `self.Box.OnComponentBeginOverlap`
  (params (OverlappedComponent :type "PrimitiveComponent Object Reference") (OtherActor :type "Actor Object Reference") (OtherComp :type "PrimitiveComponent Object Reference") (OtherBodyIndex :type Integer) (bFromSweep :type Boolean) (SweepResult :type "HitResult Structure (by ref)"))
  (set `self.bNeartheDoor` true)
  (`SceneComponent.SetVisibility` (`self.TextRender`) true false))

(event `self.Box.OnComponentEndOverlap`
  (params (OverlappedComponent :type "PrimitiveComponent Object Reference") (OtherActor :type "Actor Object Reference") (OtherComp :type "PrimitiveComponent Object Reference") (OtherBodyIndex :type Integer))
  (set `self.bNeartheDoor` false)
  (`SceneComponent.SetVisibility` (`self.TextRender`) false false))

(fn `UserConstructionScript`)